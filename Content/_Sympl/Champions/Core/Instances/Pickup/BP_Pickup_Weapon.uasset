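; Weapon pickup actor that gives a pawn the weapon referenced by its data table row handle.
; On BeginPlay it looks up the row and copies the skeletal and static meshes from the weapon class defaults onto its own components.
; TryPickup passes the row handle to the pawn's ServerEquipWeapon, then destroys the pickup without checking the result.
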(event `self.ReceiveBeginPlay`
  (bind (_datatable _rowname) (break `DataTableRowHandle` (`self.Weapon`)))
  (`parent.ReceiveBeginPlay`)
  (bind _returnvalue (`|GetDataTableRow` _datatable _rowname)
    (:`then`
      (bind _asbp_weapon (castclass `/Game/_Sympl/Champions/Core/Classes/BP_Weapon` (`.WeaponClass_6_941499314CBD4B0070D3E69A530F3E76` (break `/Game/_Sympl/Champions/Core/FWeapon` _returnvalue))))
      (bind (_mesh_sk _mesh_sm) (defaults `Object` _asbp_weapon))
      (`SkinnedMeshComponent.SetSkinnedAssetAndUpdate` (`self.SkeletalMesh`) _mesh_sk true)
      (`StaticMeshComponent.SetStaticMesh` (`self.StaticMesh`) _mesh_sm))))

(fn `TryPickup`
  (params (Pawn :type "/Game/_Sympl/Champions/Core/Classes/ChampionsPawn Object Reference"))
  (`/Game/_Sympl/Champions/Core/Classes/ChampionsPawn.Server_EquipWeapon` Pawn (`self.Weapon`))
  (`self.K2_DestroyActor`))

(fn `UserConstructionScript`
  (`parent.UserConstructionScript`))