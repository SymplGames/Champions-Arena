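; BP_Weapon is a base weapon actor that passes its attack configuration to the champion pawn wielding it.
; On BeginPlay it casts its instigator to ChampionsPawn and calls ServerUpdateCombatParams with its attack class, animation, FX, rate and shot pattern settings (pellets, arc, burst).
; The construction script caches the first component tagged AttackFXComponent as the attachment component for attack effects.
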(event `self.ReceiveBeginPlay`
  (`parent.ReceiveBeginPlay`)
  (`self.UpdateInstigatorCombatParams`))

(fn `AutoUpdateAttackFXComponent`
  (`self.UpdateAttackFXComponent` (`|GetArrayItem` (`self.GetComponentsByTag` "/Script/Engine.SceneComponent" "AttackFXComponent"))))

(fn `UpdateAttackFXComponent`
  (params (AttackFXComponent :type "SceneComponent Object Reference"))
  (set `self.AttackFXComponent` AttackFXComponent))

(fn `UpdateInstigatorCombatParams`
  (bind _aschampions_pawn (cast `/Game/_Sympl/Champions/Core/Classes/ChampionsPawn` (`self.GetInstigator`)))
  (`/Game/_Sympl/Champions/Core/Classes/ChampionsPawn.Server_UpdateCombatParams` _aschampions_pawn (`self.AttackActorClass`) (`self.AttackAnim`) (`self.AttackParticle`) (`self.AttackSound`) (`self.AttackRate`) (`self.AttackFXAttachSocket`) (`self.AttackParticleScale`) (`self.AttackClassOffset`) (`self.AttackFXSnapType`) (`self.AttackFXComponent`) (`self.bSingleShot`) (`self.NumPellets`) (`self.ShotArc`) (`self.bBurstFire`) (`self.BurstCount`)))

(fn `UserConstructionScript`
  (`parent.UserConstructionScript`)
  (`self.AutoUpdateAttackFXComponent`))