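; BP_Pickup is a configurable pickup actor that a ChampionsPawn collects by touching it.
; The construction script applies PickupMesh to the static mesh, which spins by Rotation each tick, unscaled by delta time.
; On box overlap, TryPickup passes FunctionID and FunctionParams to the pawn's ServerDoPickup, then destroys the actor, leaving the effect itself to the pawn.
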(event `self.ReceiveTick`
  (params (DeltaSeconds :type "Float (single-precision)"))
  (`parent.ReceiveTick` DeltaSeconds)
  (`SceneComponent.K2_AddLocalRotation` (`self.StaticMesh`) (`self.Rotation`) false false))

(event `self.Box.OnComponentBeginOverlap`
  (params (OverlappedComponent :type "PrimitiveComponent Object Reference") (OtherActor :type "Actor Object Reference") (OtherComp :type "PrimitiveComponent Object Reference") (OtherBodyIndex :type Integer) (bFromSweep :type Boolean) (SweepResult :type "HitResult Structure (by ref)"))
  (bind _aschampions_pawn (cast `/Game/_Sympl/Champions/Core/Classes/ChampionsPawn` OtherActor))
  (`self.TryPickup` _aschampions_pawn))

(fn `TryPickup`
  (params (Pawn :type "/Game/_Sympl/Champions/Core/Classes/ChampionsPawn Object Reference"))
  (`/Game/_Sympl/Champions/Core/Classes/ChampionsPawn.Server_DoPickup` Pawn (`self.FunctionID`) (`self.FunctionParams`))
  (`self.K2_DestroyActor`))

(fn `UserConstructionScript`
  (`parent.UserConstructionScript`)
  (`StaticMeshComponent.SetStaticMesh` (`self.StaticMesh`) (`self.PickupMesh`)))