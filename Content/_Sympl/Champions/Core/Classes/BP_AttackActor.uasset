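; BP_AttackActor is an attack actor that damages what its Sphere hits or overlaps, then destroys itself.
; Targets must pass CanDamage, which rejects owner, instigator and ignored actors and applies optional tag and class filters, though the tag check tests only the first tag.
; DoDamage applies radial (optionally falloff), point or plain damage and multicasts sound and emitter through NetworkFXComponent.
; DoDamageWithoutHitInfo fabricates a hit result from actor positions.
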(event `self.ReceiveBeginPlay`
  (`parent.ReceiveBeginPlay`)
  (`self.AddDamageIgnoreActor` (`self.GetInstigator`))
  (`self.AddDamageIgnoreActor` (`self.GetOwner`)))

(event `self.Sphere.OnComponentHit`
  (params (HitComponent :type "PrimitiveComponent Object Reference") (OtherActor :type "Actor Object Reference") (OtherComp :type "PrimitiveComponent Object Reference") (NormalImpulse :type "Vector Structure") (Hit :type "HitResult Structure (by ref)"))
  (`self.SwitchCanDamage` OtherActor OtherComp
    (:`True`
      (`self.DoDamage` OtherActor NormalImpulse Hit))))

(event `self.Sphere.OnComponentBeginOverlap`
  (params (OverlappedComponent :type "PrimitiveComponent Object Reference") (OtherActor :type "Actor Object Reference") (OtherComp :type "PrimitiveComponent Object Reference") (OtherBodyIndex :type Integer) (bFromSweep :type Boolean) (SweepResult :type "HitResult Structure (by ref)"))
  (`self.SwitchCanDamage` OtherActor OtherComp
    (:`True`
      (`self.DoDamage` OtherActor (`.ImpactNormal` (`GameplayStatics.BreakHitResult` SweepResult)) SweepResult))))

(fn `AddDamageIgnoreActor`
  (params (NewItem :type "Actor Object Reference (by ref)"))
  (`local.NewItem`
    (:`then`
      (`KismetArrayLibrary.Array_Add` (`self.DamageIgnoreActors`) (`local.NewItem`))
      (`PrimitiveComponent.IgnoreActorWhenMoving` (`self.Sphere`) (`local.NewItem`) true))
    (:`else`)))

(fn `CanDamage`
  (params (Actor :type "Actor Object Reference") (Component :type "ActorComponent Object Reference"))
  (returns (ReturnValue :type Boolean))
  (`local.Actor`
    (:`then`
      (if (and (!= (`self.GetOwner`) (`local.Actor`)) (!= (`self.GetInstigator`) (`local.Actor`)))
        (if (`KismetArrayLibrary.Array_Contains` (`self.DamageIgnoreActors`) (`local.Actor`))
          (return false)
          (else
            (return (and (`self.CheckTags` (`local.Actor`) (`local.Component`)) (`self.CheckClass` (`local.Actor`) (`local.Component`))))))
        (else
          (return false))))
    (:`else`
      (return false))))

(fn `CheckClass`
  (params (Actor :type "Object Object Reference") (Component :type "Object Object Reference"))
  (returns (ReturnValue :type Boolean))
  (if (> (`KismetArrayLibrary.Array_Length` (`self.DamageFilterClasses`)) 0)
    (`local.Actor`
      (:`then`
        (for _array_element (`self.DamageFilterClasses`)
          (if (`KismetMathLibrary.ClassIsChildOf` (`GameplayStatics.GetObjectClass` (`local.Actor`)) _array_element)
            (return true)))
        (return false))
      (:`else`
        (return false)))
    (else
      (return true))))

(fn `CheckTags`
  (params (Actor :type "Actor Object Reference") (Component :type "ActorComponent Object Reference"))
  (returns (ReturnValue :type Boolean))
  (if (> (`KismetArrayLibrary.Array_Length` (`self.DamageTags`)) 0)
    (`local.Actor`
      (:`then`
        (for _array_element (`self.DamageTags`)
          (return (`KismetArrayLibrary.Array_Contains` (`Actor.Tags` (`local.Actor`)) _array_element)))
        (return false))
      (:`else`
        (return false)))
    (else
      (return true))))

(fn `DamageFX`
  (params (Location :type "Vector Structure") (Rotation :type "Rotator Structure"))
  (`/Game/_Sympl/Common/Classes/BP_NetworkFXComponent.Multicast_Sound` (`self.NetworkFXComponent`) (`self.DamageSound`) (`local.Location`) (`local.Rotation`) 1.0 1.0 0.0 null null)
  (`/Game/_Sympl/Common/Classes/BP_NetworkFXComponent.Multicast_Emitter` (`self.NetworkFXComponent`) false (`self.DamageEmitter`) (`local.Location`) (`local.Rotation`) (1.0 1.0 1.0) true "None" true null "None" "KeepRelativeOffset"))

(fn `DoDamage`
  (params (DamagedActor :type "Actor Object Reference") (HitFromDirection :type "Vector Structure (by ref)") (HitInfo :type "HitResult Structure (by ref)"))
  (bind (_hitinfo_bblockinghit _hitinfo_binitialoverlap _hitinfo_time _hitinfo_distance _hitinfo_location _hitinfo_impactpoint) (`GameplayStatics.BreakHitResult` (`local.HitInfo`)))
  (bind (_hitinfo_bblockinghit_2 _hitinfo_binitialoverlap_2 _hitinfo_time_2 _hitinfo_distance_2 _hitinfo_location_2 _hitinfo_impactpoint_2 _hitinfo_normal _hitinfo_impactnormal) (`GameplayStatics.BreakHitResult` (`local.HitInfo`)))
  (`self.DamageFX` _hitinfo_impactpoint_2 (`KismetMathLibrary.Conv_VectorToRotator` _hitinfo_impactnormal))
  (if (`self.bRadialDamage`)
    (if (`self.bRadialWithFalloff`)
      (`GameplayStatics.ApplyRadialDamageWithFalloff` (`self.BaseDamage`) (* (`self.BaseDamage`) (`self.MinDamageScalar`)) _hitinfo_impactpoint (`self.DamageRadius_Inner`) (`self.DamageRadius_Outer`) (`self.DamageFalloff`) (`self.DamageType`) (`self.DamageIgnoreActors`) self (`self.GetInstigatorController`) (`self.DamagePreventionChannel`))
      (else
        (`GameplayStatics.ApplyRadialDamage` (`self.BaseDamage`) _hitinfo_impactpoint (`self.DamageRadius_Outer`) (`self.DamageType`) (`self.DamageIgnoreActors`) self (`self.GetInstigatorController`) (`self.bDoFullDamage`) (`self.DamagePreventionChannel`))))
    (elif (`self.bDoPointDamage`)
      (`GameplayStatics.ApplyPointDamage` (`local.DamagedActor`) (`self.BaseDamage`) (`local.HitFromDirection`) (`local.HitInfo`) (`self.GetInstigatorController`) self (`self.DamageType`))
      (else
        (`GameplayStatics.ApplyDamage` (`local.DamagedActor`) (`self.BaseDamage`) (`self.GetInstigatorController`) self (`self.DamageType`)))))
  (`self.K2_DestroyActor`))

(fn `DoDamageWithoutHitInfo`
  (params (DamagedActor :type "Actor Object Reference"))
  (locals (L_MyLoc :type "Vector Structure" :default (0.0 0.0 0.0)) (L_TheirLoc :type "Vector Structure" :default (0.0 0.0 0.0)) (L_LookAt :type "Vector Structure" :default (0.0 0.0 0.0)) (L_Dist :type "Float (double-precision)" :default 0.0))
  (set `local.L_MyLoc` (`self.K2_GetActorLocation`))
  (set `local.L_TheirLoc` (`self.K2_GetActorLocation` (`local.DamagedActor`)))
  (set `local.L_LookAt` (`KismetMathLibrary.Conv_RotatorToVector` (`KismetMathLibrary.FindLookAtRotation` (`local.L_MyLoc`) (`local.L_TheirLoc`))))
  (set `local.L_Dist` (`KismetMathLibrary.Abs` (`KismetMathLibrary.VSize` (- (`local.L_MyLoc`) (`local.L_TheirLoc`)))))
  (`self.DoDamage` (`local.DamagedActor`) (`local.L_LookAt`) (`GameplayStatics.MakeHitResult` true true (/ (`local.L_Dist`) (`KismetMathLibrary.VSize` (`self.GetVelocity`))) (`local.L_Dist`) (`local.L_TheirLoc`) (`local.L_TheirLoc`) (`local.L_LookAt`) (`local.L_LookAt`) null (`local.DamagedActor`) null "None" 0 0 (`local.L_MyLoc`) (`local.L_TheirLoc`))))

(fn `EmptyDamageIgnoreActors`
  (`KismetArrayLibrary.Array_Clear` (`self.DamageIgnoreActors`)))

(fn `RemoveDamageIgnoreActor`
  (params (Item :type "Actor Object Reference (by ref)"))
  (`local.Item`
    (:`then`
      (`KismetArrayLibrary.Array_RemoveItem` (`self.DamageIgnoreActors`) (`local.Item`))
      (`PrimitiveComponent.IgnoreActorWhenMoving` (`self.Sphere`) (`local.Item`) true))
    (:`else`)))

(fn `SetDamageIgnoreActors`
  (params (DamageIgnoreActors :type "Array of Actor Object Reference"))
  (set `self.DamageIgnoreActors` DamageIgnoreActors))

(fn `UserConstructionScript`
  (`parent.UserConstructionScript`))