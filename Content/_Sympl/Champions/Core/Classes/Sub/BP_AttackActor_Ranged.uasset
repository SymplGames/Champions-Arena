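; Ranged attack actor subclass for champions that acts as a projectile with configurable movement and look.
; The construction script calls the parent, then creates a dynamic material instance on the projectile mesh from the configured material and tints its Color parameter.
; On BeginPlay, after the parent runs, it copies its speed and bounce variables onto the ProjectileMovement component through UpdateProjectileProperties.
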(event `self.ReceiveBeginPlay`
  (`parent.ReceiveBeginPlay`)
  (`self.SetProjectileDefaults`))

(fn `SetProjectileDefaults`
  (`self.UpdateProjectileProperties` (`self.InitialSpeed`) (`self.MaxSpeed`) (`self.bShouldBounce`)))

(fn `UpdateProjectileProperties`
  (params (InitialSpeed :type "Float (double-precision)") (MaxSpeed :type "Float (double-precision)") (bShouldBounce :type Boolean))
  (set `ProjectileMovementComponent.InitialSpeed` InitialSpeed (`self.ProjectileMovement`))
  (set `ProjectileMovementComponent.MaxSpeed` MaxSpeed (`self.ProjectileMovement`))
  (set `ProjectileMovementComponent.bShouldBounce` bShouldBounce (`self.ProjectileMovement`)))

(fn `UserConstructionScript`
  (`parent.UserConstructionScript`)
  (bind _returnvalue (`PrimitiveComponent.CreateDynamicMaterialInstance` (`self.ProjectileMesh`) 0 (`self.ProjectileMaterial`) "None"))
  (`MaterialInstanceDynamic.SetVectorParameterValue` _returnvalue "Color" (`self.ProjectileColor`)))